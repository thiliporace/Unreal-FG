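; BP_PlayerCharacter is a 2D flipbook player character that moves with Enhanced Input and switches between walk and idle animations.
; While IA_Move triggers, a move event sets CharacterMovement velocity directly from the normalized input vector times PlayerSpeed and shows the walk flipbook.
; When the input completes or cancels, a reset event zeroes velocity, shows the idle flipbook and prints a debug "idle" string.
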(event `EnhancedInput|/Game/Input/IA_Move`
  (params (ActionValue :type "Vector2D Structure") (ElapsedSeconds :type "Float (double-precision)") (TriggeredSeconds :type "Float (double-precision)") (InputAction :type "InputAction Object Reference" :default "/Game/Input/IA_Move.IA_Move"))
  (:`Triggered`
    (`self.MovePlayer_Event` ActionValue))
  (:`Canceled`
    (`self.ResetToIdle_Event` :!label _label)
    (`KismetSystemLibrary.PrintString` "idle"))
  (:`Completed`
    (goto _label)))

(event `MovePlayer_Event`
  (params (PlayerDirVector :type "Vector2D Structure"))
  (set `MovementComponent.Velocity` (* (`KismetMathLibrary.Conv_Vector2DToVector` (`KismetMathLibrary.Normal2D` PlayerDirVector)) (`self.playerSpeed`)) (`self.CharacterMovement`))
  (`PaperFlipbookComponent.SetFlipbook` (`self.Sprite`) "/Game/Assets/Character/Flipbooks/FB_Walk.FB_Walk"))

(event `ResetToIdle_Event`
  (set `MovementComponent.Velocity` (`KismetMathLibrary.Vector_Zero`) (`self.CharacterMovement`))
  (`PaperFlipbookComponent.SetFlipbook` (`self.Sprite`) "/Game/Assets/Character/Flipbooks/FB_Idle.FB_Idle"))

(fn `UserConstructionScript`)