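; Stage camera that keeps all player characters in view on the X-Z plane, like a side-view multiplayer camera.
; Each tick it scans every BP_PlayerCharacter to update X and Z bounds, then centres on their midpoint with a slight upward offset.
; The larger on-screen span between the projected bound corners maps to a clamped Y position for zoom.
; The camera eases toward that target with VInterpTo.
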(event `self.ReceiveBeginPlay`
  (bind (_x _y _z) (`self.DetermineCameraLocation`)))

(event `self.ReceiveTick`
  (params (DeltaSeconds :type "Float (single-precision)"))
  (bind (_x _y _z) (`self.DetermineCameraLocation`))
  (`SceneComponent.K2_SetWorldLocation` (`self.Camera`) (`KismetMathLibrary.VInterpTo` (`SceneComponent.K2_GetComponentLocation` (`self.Camera`)) (`KismetMathLibrary.MakeVector` _x _y _z) DeltaSeconds 3.0) false false))

(fn `DetermineCameraLocation`
  (returns (X :type "Float (double-precision)") (Y :type "Float (double-precision)") (Z :type "Float (double-precision)"))
  (locals (LowestCameraCoord :type "Vector2D Structure") (HighestCameraCoord :type "Vector2D Structure") (FurthestVectorValue :type "Float (double-precision)"))
  (bind _returnvalue (`GameplayStatics.GetPlayerController` 0))
  (bind (_x _y) (`KismetMathLibrary.BreakVector2D` (`local.LowestCameraCoord`)))
  (bind (_x_2 _y_2) (`KismetMathLibrary.BreakVector2D` (`local.HighestCameraCoord`)))
  (bind _returnvalue_2 (`KismetMathLibrary.Abs` (- _x_2 _x)))
  (bind _returnvalue_3 (`KismetMathLibrary.Abs` (- _y_2 _y)))
  (bind _outactors (`GameplayStatics.GetAllActorsOfClass` "/Game/Blueprints/BP_PlayerCharacter.BP_PlayerCharacter_C"))
  (for _array_element _outactors
    (bind _x_3 (.x (`self.K2_GetActorLocation` _array_element)))
    (bind _z (.z (`self.K2_GetActorLocation` _array_element)))
    (if (<= _x_3 (`self.LowestX`))
      (set `self.LowestX` (`KismetMathLibrary.FTrunc` _x_3))
      (elif (>= _x_3 (`self.HighestX`))
        (set `self.HighestX` (`KismetMathLibrary.FTrunc` _x_3))))
    (if (<= _z (`self.LowestZ`))
      (set `self.LowestZ` (`KismetMathLibrary.FTrunc` _z))
      (elif (>= _z (`self.HighestZ`))
        (set `self.HighestZ` (`KismetMathLibrary.FTrunc` _z)))))
  (set `self.IdealXPosition` (/ (+ (`self.LowestX`) (`self.HighestX`)) 2))
  (set `self.IdealZPosition` (/ (+ (`self.LowestZ`) (`self.HighestZ`)) 2))
  (set `local.LowestCameraCoord` (`GameplayStatics.ProjectWorldToScreen` _returnvalue (`KismetMathLibrary.MakeVector` (`KismetMathLibrary.Conv_IntToDouble` (`self.LowestX`)) 0.0 (`KismetMathLibrary.Conv_IntToDouble` (`self.LowestZ`)))))
  (set `local.HighestCameraCoord` (`GameplayStatics.ProjectWorldToScreen` _returnvalue (`KismetMathLibrary.MakeVector` (`KismetMathLibrary.Conv_IntToDouble` (`self.HighestX`)) 0.0 (`KismetMathLibrary.Conv_IntToDouble` (`self.HighestZ`)))))
  (if (> _returnvalue_2 _returnvalue_3)
    (set `local.FurthestVectorValue` _returnvalue_2)
    (else
      (set `local.FurthestVectorValue` _returnvalue_3)))
  (return (`KismetMathLibrary.Conv_IntToDouble` (`self.IdealXPosition`)) (`KismetMathLibrary.MapRangeClamped` (`local.FurthestVectorValue`) 100.0 1800.0 100.0 1500.0) (+ (`KismetMathLibrary.Conv_IntToDouble` (`self.IdealZPosition`)) 100.0)))

(fn `UserConstructionScript`)